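; Master game mode that runs a match through Waiting, Battle and Ceremony states on a looping one-second timer.
; Waiting counts down once enough players join, broadcasting status through each controller's notification string; late joiners get removed via a short lifespan.
; Battle updates the GameState alive count but declares the first player winner whenever at least one remains.
; The death event is empty, with its result and list-update logic left disconnected.
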(event `self.ReceiveBeginPlay`
  (bind _returnvalue (`KismetSystemLibrary.K2_SetTimerDelegate` (delegate `MainTimer`) 1.0 true))
  (set `self.MainTimerHandle` _returnvalue))

(event `MainTimer`
  (bind _alivepcs (`self.AlivePCs`))
  (bind _remaintimetostart (`self.RemainTimetoStart`))
  (switch `/Game/02_GameMode_Controller/EPlayingState` (`self.PlayingState`)
    (:`NewEnumerator0`
      ;[1 1 1] Waiting
      (if (>= (`KismetArrayLibrary.Array_Length` (`self.AlivePCs`)) (`self.MinimunPlayerCount`))
        (bind _result (`/Engine/EditorBlueprintResources/StandardMacros.DecrementInt` _remaintimetostart)
          (:`  `
            (if (== _result 0)
              (`|ExecutionSequence`
                (:`then_0`
                  (set `self.PlayingState` "NewEnumerator1"))
                (:`then_1`
                  (`self.SayToAll` "Starting the Battle.")
                  (`KismetSystemLibrary.Delay` 5.0)
                  (`self.SayToAll` "")))
              (else
                (`self.SayToAll` (`KismetTextLibrary.Conv_TextToString` (`|FormatText` "{T}sec Left before the Battle" _remaintimetostart)))))))
        (else
          (set `self.RemainTimetoStart` (`self.WatingTime`))
          (`self.SayToAll` "Waiting for other players..."))))
    (:`NewEnumerator1`
      (bind _asbp_game_state (cast `/Game/02_GameMode_Controller/BP_GameState` (`GameplayStatics.GetGameState`)))
      (bind _output_get (set `/Game/02_GameMode_Controller/BP_GameState.AliveCount` (`KismetArrayLibrary.Array_Length` _alivepcs) _asbp_game_state))
      (if (>= _output_get 1)
        (`/Game/02_GameMode_Controller/BP_PlayerControllerMaster.ShowWinnerResult` (`|GetArrayItem` _alivepcs))
        (set `self.PlayingState` "NewEnumerator2")))
    (:`NewEnumerator2`
      (`self.SayToAll` "Battle Finish!"))))

(event `OnCharcterDeath`
  (params (PlayerController :type "/Game/02_GameMode_Controller/BP_PlayerControllerMaster Object Reference"))
  ;[1 1 1] Players Death
)

(event `self.K2_PostLogin`
  (params (NewPlayer :type "PlayerController Object Reference"))
  ;[1 1 1] Log in/out
  (bind _asbp_player_controller_master (cast `/Game/02_GameMode_Controller/BP_PlayerControllerMaster` NewPlayer))
  (if (`|EnumEquality` (`self.PlayingState`) "NewEnumerator0")
    (`KismetArrayLibrary.Array_Add` (`self.AlivePCs`) _asbp_player_controller_master)
    (set `/Game/02_GameMode_Controller/BP_PlayerControllerMaster.NotificationFromServer` "You will be moved to a Flight Soon!" _asbp_player_controller_master)
    (else
      (`self.SetLifeSpan` _asbp_player_controller_master 0.1) ; 만약 waiting 상태가 아니면 접속을 끊는다
    )))

(event `self.K2_OnLogout`
  (params (ExitingController :type "Controller Object Reference"))
  ;[1 1 1] Log in/out
  (bind _asbp_player_controller_master (cast `/Game/02_GameMode_Controller/BP_PlayerControllerMaster` ExitingController))
  (`KismetArrayLibrary.Array_RemoveItem` (`self.AlivePCs`) _asbp_player_controller_master))

(fn `SayToAll`
  (params (Message :type String))
  (for _array_element (`self.AlivePCs`)
    (set `/Game/02_GameMode_Controller/BP_PlayerControllerMaster.NotificationFromServer` Message _array_element)))

(fn `UserConstructionScript`)