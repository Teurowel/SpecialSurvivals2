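; Master player controller that manages the main client HUD and end-of-match results for a ranked, "chicken dinner" style battle match.
; On BeginPlay, only the non-authority side creates WBP_ClientMain, passing it the controller and BP_GameState.
; Character death is forwarded to GM_GameModeMaster.
; Separate death and winner events show WBP_BattleResults with a Korean message and either the given rank or first place.
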(event `self.ReceiveBeginPlay`
  (`/Engine/EditorBlueprintResources/ActorMacros.Switch Has Authority` ; 이 BeginPlay가 내 클라에서 실행되는지, 아니면 서버에서 실행되는지를 가려주는 노드 / Authority - Server, Remote - Client
    (:`Remote`
      (bind _asbp_game_state (cast `/Game/02_GameMode_Controller/BP_GameState` (`GameplayStatics.GetGameState`)))
      (bind _returnvalue (`|CreateWidget` "/Game/03_HUD/WBP_ClientMain.WBP_ClientMain_C" self self _asbp_game_state))
      (`UserWidget.AddToViewport` _returnvalue 0))))

(event `OnCharacterDeath`
  (bind _returnvalue (`GameplayStatics.GetGameMode`))
  (`/Engine/EditorBlueprintResources/StandardMacros.IsValid` _returnvalue
    (:`Is Valid`
      (bind _asgm_game_mode_master (cast `/Game/02_GameMode_Controller/GM_GameModeMaster` _returnvalue))
      (`/Game/02_GameMode_Controller/GM_GameModeMaster.OnCharcterDeath` _asgm_game_mode_master self))))

(event `ShowDeathResult`
  (params (Rank :type Integer))
  (bind _returnvalue (`|CreateWidget` "/Game/03_HUD/WBP_BattleResults.WBP_BattleResults_C" self "졌닭, 치킨은 다음에!" (`KismetStringLibrary.Concat_StrStr` "#" (`KismetStringLibrary.Conv_IntToString` Rank))))
  (`UserWidget.AddToViewport` _returnvalue 0))

(event `ShowWinnerResult`
  (bind _returnvalue (`|CreateWidget` "/Game/03_HUD/WBP_BattleResults.WBP_BattleResults_C" null "이겼닭, 오늘 저녁은 치킨이닭!" "#1"))
  (`UserWidget.AddToViewport` _returnvalue 0))

(fn `UserConstructionScript`)