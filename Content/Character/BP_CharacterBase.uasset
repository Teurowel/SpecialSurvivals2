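; BP_CharacterBase is a character base holding weapon pickup, hitscan firing, health and death logic.
; Overlap functions track a candidate BP_WeaponBase, which pickup attaches to the hand socket after detaching any equipped one.
; Firing spends ammo, plays effects and line-traces from the camera to damage characters, clearing its timer when empty.
; Death disables input and capsule collision, plays an animation and notifies BP_PlayerControllerMaster.
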(fn `CheckWeaponBeginOverlap`
  (params (OtherActor :type "Actor Object Reference"))
  (bind _asbp_weapon_base (cast `/Game/Weapon/BP_WeaponBase` OtherActor))
  (if (not (== (`self.EquippedWeapon`) _asbp_weapon_base))
    (bind _output_get (set `self.OverlappedWeapon` _asbp_weapon_base))
    (`KismetSystemLibrary.PrintString` (`KismetSystemLibrary.GetDisplayName` _output_get))))

(fn `CheckWeaponEndOverlap`
  (params (OtherActor :type "Actor Object Reference"))
  (bind _asbp_weapon_base (cast `/Game/Weapon/BP_WeaponBase` OtherActor))
  (if (not (== _asbp_weapon_base (`self.EquippedWeapon`)))
    (set `self.OverlappedWeapon` null)
    (`KismetSystemLibrary.PrintString` "No overlap")))

(fn `DeathCheck`
  (if (<= (`self.Health`) 0.0)
    (`self.DisableInput` (`GameplayStatics.GetPlayerController` 0))
    (`SkeletalMeshComponent.PlayAnimation` (`self.Mesh`) "/Game/Character/Player1/Animation/death_from_the_front.death_from_the_front" false)
    (`PrimitiveComponent.SetCollisionEnabled` (`self.CapsuleComponent`) "NoCollision")
    (bind _asbp_player_controller_master (cast `/Game/02_GameMode_Controller/BP_PlayerControllerMaster` (`self.GetController`)))
    (`/Game/02_GameMode_Controller/BP_PlayerControllerMaster.OnCharacterDeath` _asbp_player_controller_master)))

(fn `DecreaseHealth`
  (params (Damage :type "Float (double-precision)"))
  (bind _output_get (set `self.Health` (- (`self.Health`) Damage)))
  (`KismetSystemLibrary.PrintString` (`KismetStringLibrary.Conv_DoubleToString` _output_get)))

(fn `FireWeapon`
  (bind _camera (`self.Camera`))
  (bind _returnvalue (`SceneComponent.K2_GetComponentLocation` _camera))
  ;[1 1 1] Check Ammo
  (if (> (`/Game/Weapon/BP_WeaponBase.Ammo` (`self.EquippedWeapon`)) 0)
    ;[1 1 1] Decrease Ammo
    (`/Engine/EditorBlueprintResources/StandardMacros.DecrementInt` (`/Game/Weapon/BP_WeaponBase.Ammo` (`self.EquippedWeapon`))
      (:`  `
        ;[1 1 1] Create MuzzleFlash
        (`GameplayStatics.SpawnEmitterAttached` "/Game/Effects/P_WeaponMuzzleFlash.P_WeaponMuzzleFlash" (`/Game/Weapon/BP_WeaponBase.SkeletalMesh` (`self.EquippedWeapon`)) "MuzzleFlashSocket")
        (`GameplayStatics.SpawnSoundAttached` "/Game/Sound/Weapons/SMG_Thompson/Cue_Thompson_Shot.Cue_Thompson_Shot" (`self.Mesh`) "None" (0.0 0.0 0.0) (struct) "KeepRelativeOffset" false 1.0 1.0 0.0 null null)
        ;[1 1 1] LineTrace
        (bind _outhit (`KismetSystemLibrary.LineTraceSingle` :`Start` _returnvalue :`End` (+ _returnvalue (* (`KismetMathLibrary.GetForwardVector` (`SceneComponent.K2_GetComponentRotation` _camera)) (`/Game/Weapon/BP_WeaponBase.Range` (`self.EquippedWeapon`)))) :`TraceChannel` "TraceTypeQuery1" :`DrawDebugType` "ForDuration"))
        ;[1 1 1] Deal Damage To Character
        (bind _asbp_character_base (cast `/Game/Character/BP_CharacterBase` (`.HitActor` (`GameplayStatics.BreakHitResult` _outhit))))
        (`self.DecreaseHealth` _asbp_character_base (`/Game/Weapon/BP_WeaponBase.Damage` (`self.EquippedWeapon`)))
        ;[1 1 1] Death Check
        (`self.DeathCheck` _asbp_character_base)))
    (else
      (`KismetSystemLibrary.K2_ClearTimer` null "FireWeapon"))))

(fn `PickupWeapon`
  (`/Engine/EditorBlueprintResources/StandardMacros.IsValid` (`self.OverlappedWeapon`)
    (:`Is Valid`
      (`KismetSystemLibrary.PrintString` "picked up!")
      (`/Engine/EditorBlueprintResources/StandardMacros.IsValid` (`self.EquippedWeapon`)
        (:`Is Valid`
          (`/Game/Weapon/BP_WeaponBase.DetachFromCharacter` (`self.EquippedWeapon`) (`self.GetTransform` (`self.OverlappedWeapon`))))
        (:`Is Not Valid`
          _))
      (set `self.EquippedWeapon` (`self.OverlappedWeapon`))
      (`/Game/Weapon/BP_WeaponBase.AttachToCharacter` (`self.OverlappedWeapon`) (`self.Mesh`) "WeaponSocket")
      (set `self.OverlappedWeapon` null))
    (:`Is Not Valid`
      (`KismetSystemLibrary.PrintString` "No pickup"))))

(fn `UserConstructionScript`)