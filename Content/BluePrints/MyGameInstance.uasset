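; MyGameInstance is a Game Instance Blueprint that shows and hides the options HUD.
; ShowOptionHUD creates the HUD_Option widget on first use, caches it and adds it to the viewport; later calls reuse it by making it visible.
; CloseOptionHUD collapses the cached widget instead of removing it, without checking that it exists.
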(fn `CloseOptionHUD`
  (`Widget.SetVisibility` (`self.HUD_Option`) "Collapsed"))

(fn `ShowOptionHUD`
  (`/Engine/EditorBlueprintResources/StandardMacros.IsValid` (`self.HUD_Option`)
    (:`Is Valid`
      (`Widget.SetVisibility` (`self.HUD_Option`) "Visible"))
    (:`Is Not Valid`
      ;[1 1 1] Create Option HUD
      (bind _returnvalue (`|CreateWidget` "/Game/03_HUD/HUD_Option.HUD_Option_C"))
      (bind _output_get (set `self.HUD_Option` _returnvalue))
      (`UserWidget.AddToViewport` _output_get 1)
      (`Widget.SetVisibility` _output_get "Visible"))))